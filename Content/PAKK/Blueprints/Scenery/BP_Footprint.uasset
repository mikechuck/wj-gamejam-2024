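; BP_Footprint is a scenery footprint decal that shows only while something is within range.
; Overlaps on its RenderTrigger component show and hide the decal, with no filter on the overlapping actor.
; On BeginPlay it also shows the decal if GM_Gameplay's PackSpawnLocation lies within the trigger's bounds radius plus a fixed margin, covering footprints near the player's spawn.
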(event `self.ReceiveBeginPlay`
  ;[1 1 1] Set footprint to visible if near player at spawn
  (bind _asgm_gameplay (cast `/Game/PAKK/GM_Gameplay` (`GameplayStatics.GetGameMode`)))
  (if (<= (`KismetMathLibrary.Vector_Distance` (`SceneComponent.K2_GetComponentLocation` (`self.Decal`)) (`/Game/PAKK/GM_Gameplay.PackSpawnLocation` _asgm_gameplay)) (+ (`.SphereRadius` (`KismetSystemLibrary.GetComponentBounds` (`self.RenderTrigger`))) 500.0))
    (`SceneComponent.SetVisibility` (`self.Decal`) true false)))

(event `self.RenderTrigger.OnComponentBeginOverlap`
  (params (OverlappedComponent :type "PrimitiveComponent Object Reference") (OtherActor :type "Actor Object Reference") (OtherComp :type "PrimitiveComponent Object Reference") (OtherBodyIndex :type Integer) (bFromSweep :type Boolean) (SweepResult :type "HitResult Structure (by ref)"))
  (`SceneComponent.SetVisibility` (`self.Decal`) true false))

(event `self.RenderTrigger.OnComponentEndOverlap`
  (params (OverlappedComponent :type "PrimitiveComponent Object Reference") (OtherActor :type "Actor Object Reference") (OtherComp :type "PrimitiveComponent Object Reference") (OtherBodyIndex :type Integer))
  (`SceneComponent.SetVisibility` (`self.Decal`) false false))

(fn `UserConstructionScript`)