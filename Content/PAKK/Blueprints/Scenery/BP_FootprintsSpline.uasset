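; Scenery actor that lays five wandering trails of footprint decals between the pack and camp spawn locations read from GM_Gameplay.
; Its construction script sets each spline's endpoints, then inserts randomly Y-offset intermediate points, with the other four splines jittered around the first.
; Decals are spawned at fixed intervals along each spline, alternating world-Y offset and flipped rotation for left and right feet.
; The ground-snapping function is disconnected and never called.
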(fn `CreateFootprints`
  (params (Spline :type "SplineComponent Object Reference"))
  (locals (SplineVal :type "SplineComponent Object Reference") (SplineIndex :type Integer) (DecalComponent :type "DecalComponent Object Reference") (DecalYOffset :type "Float (double-precision)"))
  (bind _returnvalue (* (mod (`local.SplineIndex`) 2) 180))
  (bind (_returnvalue_x _returnvalue_y _returnvalue_z) (`KismetMathLibrary.BreakVector` (`SplineComponent.GetLocationAtDistanceAlongSpline` (`local.SplineVal`) (`KismetMathLibrary.Conv_IntToDouble` (* (`local.SplineIndex`) 50)) "World")))
  (bind (_returnvalue_roll _returnvalue_pitch _returnvalue_yaw) (`KismetMathLibrary.BreakRotator` (`SplineComponent.GetRotationAtDistanceAlongSpline` (`local.SplineVal`) (`KismetMathLibrary.Conv_IntToDouble` (* (`local.SplineIndex`) 50)) "World")))
  (set `local.SplineVal` Spline)
  ;[0.3698 0.3698 0.3698] Create footprint decals for both feet along path
  ;;[1 1 1] Create new decal component with all the spawn data
  (for _index (range (+ (`KismetMathLibrary.FTrunc` (/ (`SplineComponent.GetSplineLength` (`local.SplineVal`)) 50.0)) 1))
    (set `local.SplineIndex` _index)
    (bind _returnvalue_2 (`AddComponent|NODE_AddDecalComponent-2` :`RelativeTransform` (`KismetMathLibrary.MakeTransform` (0.0 0.0 0.0) (struct :`Pitch` 90.0) (25.0 1.0 1.0))))
    (set `local.DecalComponent` _returnvalue_2)
    (set `local.DecalYOffset` _returnvalue_y)
    ;;[1 1 1] Change decal distance from center line based on which foot
    (if (== (mod (`local.SplineIndex`) 2) 0)
      (set `local.DecalYOffset` (+ (`local.DecalYOffset`) (`self.GateWidth`)))
      (else
        (set `local.DecalYOffset` (- (`local.DecalYOffset`) (`self.GateWidth`)))))
    (`SceneComponent.K2_SetWorldLocationAndRotation` (`local.DecalComponent`) (`KismetMathLibrary.MakeVector` _returnvalue_x (`local.DecalYOffset`) _returnvalue_z) (`KismetMathLibrary.MakeRotator` (- _returnvalue_roll _returnvalue 90.0) (+ _returnvalue _returnvalue_pitch 90.0) _returnvalue_yaw) false false)
    (`DecalComponent.SetDecalMaterial` (`local.DecalComponent`) (`self.FootDecal`))))

(fn `SetupSplinePoints`
  (locals (PackSpawnLocation :type "Vector Structure") (CampSpawnLocation :type "Vector Structure") (NewPointLocation :type "Vector Structure") (SpineIndex :type Integer))
  (bind (_campspawnlocation_x _campspawnlocation_y _campspawnlocation_z) (`KismetMathLibrary.BreakVector` (`local.CampSpawnLocation`)))
  (bind (_packspawnlocation_x _packspawnlocation_y _packspawnlocation_z) (`KismetMathLibrary.BreakVector` (`local.PackSpawnLocation`)))
  (bind _numsplinesections (`self.NumSplineSections`))
  (bind _spineindex (`local.SpineIndex`))
  (bind (_campspawnlocation_x_2 _campspawnlocation_y_2 _campspawnlocation_z_2) (`KismetMathLibrary.BreakVector` (`local.CampSpawnLocation`)))
  (bind (_campspawnlocation_x_3 _campspawnlocation_y_3 _campspawnlocation_z_3) (`KismetMathLibrary.BreakVector` (`local.CampSpawnLocation`)))
  (bind (_packspawnlocation_x_2 _packspawnlocation_y_2 _packspawnlocation_z_2) (`KismetMathLibrary.BreakVector` (`local.PackSpawnLocation`)))
  (bind (_campspawnlocation_x_4 _campspawnlocation_y_4 _campspawnlocation_z_4) (`KismetMathLibrary.BreakVector` (`local.CampSpawnLocation`)))
  (bind (_packspawnlocation_x_3 _packspawnlocation_y_3 _packspawnlocation_z_3) (`KismetMathLibrary.BreakVector` (`local.PackSpawnLocation`)))
  (bind (_campspawnlocation_x_5 _campspawnlocation_y_5 _campspawnlocation_z_5) (`KismetMathLibrary.BreakVector` (`local.CampSpawnLocation`)))
  (bind (_packspawnlocation_x_4 _packspawnlocation_y_4 _packspawnlocation_z_4) (`KismetMathLibrary.BreakVector` (`local.PackSpawnLocation`)))
  (bind (_packspawnlocation_x_5 _packspawnlocation_y_5 _packspawnlocation_z_5) (`KismetMathLibrary.BreakVector` (`local.PackSpawnLocation`)))
  (bind _returnvalue (- _campspawnlocation_x_3 _packspawnlocation_x_2))
  (bind _returnvalue_2 (- _campspawnlocation_y_3 _packspawnlocation_y_2))
  (bind _returnvalue_3 (- _campspawnlocation_z_3 _packspawnlocation_z_2))
  ;[1 1 1] Get Game mode variables
  (bind _asgm_gameplay (cast `/Game/PAKK/GM_Gameplay` (`GameplayStatics.GetGameMode`)))
  (set `local.PackSpawnLocation` (`/Game/PAKK/GM_Gameplay.PackSpawnLocation` _asgm_gameplay))
  (set `local.CampSpawnLocation` (`/Game/PAKK/GM_Gameplay.CampSpawnLocation` _asgm_gameplay))
  (`|ExecutionSequence`
    (:`then_0`
      ;[1 1 1] Set both ends of spline to both spawn points
      (`SplineComponent.SetLocationAtSplinePoint` (`self.Spline1`) 0 (`local.PackSpawnLocation`) "World" true)
      (`SplineComponent.SetLocationAtSplinePoint` (`self.Spline1`) 1 (`local.CampSpawnLocation`) "World" true))
    (:`then_1`
      ;[1 1 1] Set both ends of spline to both spawn points
      (`SplineComponent.SetLocationAtSplinePoint` (`self.Spline2`) 0 (+ (`local.PackSpawnLocation`) (`self.Spline2StartPos`)) "World" true)
      (`SplineComponent.SetLocationAtSplinePoint` (`self.Spline2`) 1 (+ (`local.CampSpawnLocation`) (`self.Spline2StartPos`)) "World" true))
    (:`then_2`
      ;[1 1 1] Set both ends of spline to both spawn points
      (`SplineComponent.SetLocationAtSplinePoint` (`self.Spline3`) 0 (+ (`local.PackSpawnLocation`) (`self.Spline3StartPos`)) "World" true)
      (`SplineComponent.SetLocationAtSplinePoint` (`self.Spline3`) 1 (+ (`local.CampSpawnLocation`) (`self.Spline3StartPos`)) "World" true))
    (:`then_3`
      ;[1 1 1] Set both ends of spline to both spawn points
      (`SplineComponent.SetLocationAtSplinePoint` (`self.Spline4`) 0 (+ (`local.PackSpawnLocation`) (`self.Spline4StartPos`)) "World" true)
      (`SplineComponent.SetLocationAtSplinePoint` (`self.Spline4`) 1 (+ (`local.CampSpawnLocation`) (`self.Spline4StartPos`)) "World" true))
    (:`then_4`
      ;[1 1 1] Set both ends of spline to both spawn points
      (`SplineComponent.SetLocationAtSplinePoint` (`self.Spline5`) 0 (+ (`local.PackSpawnLocation`) (`self.Spline4StartPos`)) "World" true)
      (`SplineComponent.SetLocationAtSplinePoint` (`self.Spline5`) 1 (+ (`local.CampSpawnLocation`) (`self.Spline4StartPos`)) "World" true))
    (:`then_5`
      (for _index (range 1 (`self.NumSplineSections`))
        (set `local.SpineIndex` _index)
        (`|ExecutionSequence`
          (:`then_0`
            ;[1 1 1] Create path spline points all the way to camp
            (bind _output_get (set `self.MainSplinePointLocation` (+ (`KismetMathLibrary.MakeVector` (+ (/ (* _returnvalue _spineindex) _numsplinesections) _packspawnlocation_x_2) (+ (/ (* _returnvalue_2 _spineindex) _numsplinesections) _packspawnlocation_y_2) (+ (/ (* _returnvalue_3 _spineindex) _numsplinesections) _packspawnlocation_z_2)) (* (`KismetMathLibrary.Normal` (`KismetMathLibrary.MakeVector` _returnvalue _returnvalue_2 _returnvalue_3)) (`KismetMathLibrary.MakeVector` 0.0 (* (`KismetMathLibrary.RandomFloatInRange` -1.0 1.0) 15000.0))))))
            (`SplineComponent.AddSplinePointAtIndex` (`self.Spline1`) _output_get (`local.SpineIndex`) "World" true))
          (:`then_1`
            ;[1 1 1] Setup spline 1 points
            (`SplineComponent.AddSplinePointAtIndex` (`self.Spline2`) (+ (`self.MainSplinePointLocation`) (* (`KismetMathLibrary.Normal` (`KismetMathLibrary.MakeVector` (- _campspawnlocation_x_4 _packspawnlocation_x_3) (- _campspawnlocation_y_4 _packspawnlocation_y_3) (- _campspawnlocation_z_4 _packspawnlocation_z_3))) (`KismetMathLibrary.MakeVector` 0.0 (`KismetMathLibrary.RandomFloatInRange` -500.0 500.0)))) (`local.SpineIndex`) "World" true))
          (:`then_2`
            ;[1 1 1] Setup spline 2 points
            (`SplineComponent.AddSplinePointAtIndex` (`self.Spline3`) (+ (`self.MainSplinePointLocation`) (* (`KismetMathLibrary.Normal` (`KismetMathLibrary.MakeVector` (- _campspawnlocation_x_5 _packspawnlocation_x_4) (- _campspawnlocation_y_5 _packspawnlocation_y_4) (- _campspawnlocation_z_5 _packspawnlocation_z_4))) (`KismetMathLibrary.MakeVector` 0.0 (`KismetMathLibrary.RandomFloatInRange` -1000.0 1000.0)))) (`local.SpineIndex`) "World" true))
          (:`then_3`
            ;[1 1 1] Setup spline 3 points
            (`SplineComponent.AddSplinePointAtIndex` (`self.Spline4`) (+ (`self.MainSplinePointLocation`) (* (`KismetMathLibrary.Normal` (`KismetMathLibrary.MakeVector` (- _campspawnlocation_x _packspawnlocation_x) (- _campspawnlocation_y _packspawnlocation_y) (- _campspawnlocation_z _packspawnlocation_z))) (`KismetMathLibrary.MakeVector` 0.0 (`KismetMathLibrary.RandomFloatInRange` -1000.0 1000.0)))) (`local.SpineIndex`) "World" true))
          (:`then_4`
            ;[1 1 1] Setup spline 3 points
            (`SplineComponent.AddSplinePointAtIndex` (`self.Spline5`) (+ (`self.MainSplinePointLocation`) (* (`KismetMathLibrary.Normal` (`KismetMathLibrary.MakeVector` (- _campspawnlocation_x_2 _packspawnlocation_x_5) (- _campspawnlocation_y_2 _packspawnlocation_y_5) (- _campspawnlocation_z_2 _packspawnlocation_z_5))) (`KismetMathLibrary.MakeVector` 0.0 (`KismetMathLibrary.RandomFloatInRange` -1000.0 1000.0)))) (`local.SpineIndex`) "World" true)))))))

(fn `SnapPointsToGround`
  (params (Spline :type "SplineComponent Object Reference"))
  (locals (SplineVal :type "SplineComponent Object Reference"))
  ;[1 1 1] Snap spline points to ground
  (bind _output_get (set `local.SplineVal` Spline)))

(fn `UserConstructionScript`
  (locals (SplineIndex :type Integer) (DecalComponent :type "DecalComponent Object Reference") (DecalYOffset :type "Float (double-precision)" :default 0.0) (GameMode :type "/Game/PAKK/GM_Gameplay Object Reference") (LatestSplinePoint :type "Vector Structure") (CampSpawnLocation :type "Vector Structure" :default (0.0 0.0 0.0)) (PackSpawnLocation :type "Vector Structure"))
  (`self.SetupSplinePoints`)
  (`self.CreateFootprints` (`self.Spline1`))
  (`self.CreateFootprints` (`self.Spline2`))
  (`self.CreateFootprints` (`self.Spline3`))
  (`self.CreateFootprints` (`self.Spline4`))
  (`self.CreateFootprints` (`self.Spline5`)))