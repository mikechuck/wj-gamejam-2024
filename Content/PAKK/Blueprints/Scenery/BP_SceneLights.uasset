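; BP_SceneLights is a scenery Blueprint that gradually dims the scene's directional light and thickens its height fog during play.
; BeginPlay applies the starting intensity and fog density, then starts a looping timer on DecreaseLight after an initial delay.
; Each tick of that timer steps intensity down toward a minimum and fog density up toward a maximum, despite a graph comment labelling the fog step as light temperature.
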(event `self.ReceiveBeginPlay`
  (`KismetSystemLibrary.K2_SetTimer` null "DecreaseLight" 1.0 true 15.0)
  (`LightComponent.SetIntensity` (`self.DirectionalLight`) (`self.LightIntensity`))
  (`ExponentialHeightFogComponent.SetFogDensity` (`self.ExponentialHeightFog`) (`self.FogLevel`)))

(fn `DecreaseLight`
  (`|ExecutionSequence`
    (:`then_0`
      ;[1 1 1] Change light intensity
      (if (>= (`self.LightIntensity`) (`self.MinLightIntensity`))
        (bind _output_get (set `self.LightIntensity` (- (`self.LightIntensity`) 0.025)))
        (`LightComponent.SetIntensity` (`self.DirectionalLight`) _output_get)))
    (:`then_2`
      ;[1 1 1] Change light temperature
      (if (< (`self.FogLevel`) (`self.MaxFogLevel`))
        (set `self.FogLevel` (+ (`self.FogLevel`) 0.05))
        (`ExponentialHeightFogComponent.SetFogDensity` (`self.ExponentialHeightFog`) (`self.FogLevel`))))))

(fn `UserConstructionScript`)