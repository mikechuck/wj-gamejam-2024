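; Gameplay game mode that sets up the level at BeginPlay and drives timed events once NPC following is enabled.
; It finds tagged spawn points, spawns four NPCs, a footprint spline at the pack spawn and scene lights, adds the HUD, and enables player controls after a delay.
; An enable-NPC dispatcher relays to a second one and starts a Tick-driven run timer.
; Timed events are stubs: a debug print and unused tree traces.
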(event `SetGmEnableNpc_Event`
  ;[1 1 1] Custom event handlers
  (`self.SetBpEnableNpc`)
  (set `self.EnableNpcFollow` true))

(event `self.ReceiveBeginPlay`
  (`|ExecutionSequence`
    (:`then_0`
      (`self.CreateSpawnAreas`))
    (:`then_1`
      (`self.SpawnNPCs`))
    (:`then_2`
      (`self.SpawnFootprints`))
    (:`then_3`
      ;[1 1 1] Custom event handlers
      (add `self.SetGmEnableNpc` (delegate `SetGmEnableNpc_Event`)))
    (:`then_4`
      ;[1 1 1] Setup UI
      (bind _returnvalue (`|CreateWidget` "/Game/PAKK/UI/WB_PlayerHud.WB_PlayerHud_C"))
      (bind _output_get (set `self.PlayerHud` _returnvalue))
      (`UserWidget.AddToPlayerScreen` _output_get 0))
    (:`then_5`
      ;[1 1 1] Enable player controls after delay
      (`KismetSystemLibrary.Delay` 15.0)
      (bind _asbp_player_controller (cast `/Game/PAKK/Blueprints/Players/Player/BP_PlayerController` (`GameplayStatics.GetPlayerController` 0)))
      (`/Game/PAKK/Blueprints/Players/Player/BP_PlayerController.EnableControls` _asbp_player_controller))
    (:`then_6`
      ;[1 1 1] Spawn light blueprint
      (`|SpawnActorFromClass` "/Game/PAKK/Blueprints/Scenery/BP_SceneLights.BP_SceneLights_C" (`KismetMathLibrary.MakeTransform` (0.0 0.0 0.0) (struct :`Pitch` -20.0)) "Undefined" "MultiplyWithRoot" null null))))

(event `self.ReceiveTick`
  (params (DeltaSeconds :type "Float (single-precision)"))
  ;[1 1 1] Update runtime if player has left start area
  (if (`self.EnableNpcFollow`)
    (set `self.RunTime` (+ (`self.RunTime`) DeltaSeconds))
    (`self.HandleRunTimeEvents`)))

(fn `CreateSpawnAreas`
  ;[1 1 1] Initiate spawn locations
  (bind _outactors (`GameplayStatics.GetAllActorsWithTag` "CampSpawn"))
  (set `self.CampSpawnLocation` (`self.K2_GetActorLocation` (`|GetArrayItem` _outactors)))
  (bind _outactors_2 (`GameplayStatics.GetAllActorsWithTag` "PackSpawn"))
  (set `self.PackSpawnLocation` (`self.K2_GetActorLocation` (`|GetArrayItem` _outactors_2))))

(fn `HandleRunTimeEvents`
  (bind _returnvalue (`self.K2_GetActorLocation` (`GameplayStatics.GetPlayerCharacter` 0)))
  (`|ExecutionSequence`
    (:`then_0`
      ;[1 1 1] Run Event1
      (if (and (> (`self.RunTime`) 5.0) (not (`self.HasEvent1Run`)))
        (set `self.HasEvent1Run` true)
        (`KismetSystemLibrary.PrintString` "Running event 1")))
    (:`then_1`
      (for _ (range 7)
        (bind (_outhit _returnvalue_2) (`KismetSystemLibrary.LineTraceSingleForObjects` _returnvalue (+ _returnvalue (100.0 100.0 0.0)) (`self.TreeMeshes`)))
        (if _returnvalue_2
          _)))))

(fn `SpawnFootprints`
  ;[1 1 1] Spawn footprint paths
  (`|SpawnActorFromClass` "/Game/PAKK/Blueprints/Scenery/BP_FootprintsSpline.BP_FootprintsSpline_C" (`KismetMathLibrary.MakeTransform` (`self.PackSpawnLocation`)) "Undefined" "MultiplyWithRoot" null null))

(fn `SpawnNPCs`
  (`|ExecutionSequence`
    (:`then_0`
      (`|SpawnActorFromClass` "/Game/PAKK/Blueprints/Players/NPC/BP_NpcAI.BP_NpcAI_C" (`KismetMathLibrary.MakeTransform` (+ (`KismetMathLibrary.MakeVector` 40.0 -30.0 50.0) (`self.PackSpawnLocation`)) (struct :`Yaw` 150.0)) "AdjustIfPossibleButAlwaysSpawn" "MultiplyWithRoot" null null))
    (:`then_1`
      (`|SpawnActorFromClass` "/Game/PAKK/Blueprints/Players/NPC/BP_NpcAI.BP_NpcAI_C" (`KismetMathLibrary.MakeTransform` (+ (`KismetMathLibrary.MakeVector` 290.0 410.0 50.0) (`self.PackSpawnLocation`)) (struct :`Yaw` -50.0)) "AdjustIfPossibleButAlwaysSpawn" "MultiplyWithRoot" null null))
    (:`then_2`
      (`|SpawnActorFromClass` "/Game/PAKK/Blueprints/Players/NPC/BP_NpcAI.BP_NpcAI_C" (`KismetMathLibrary.MakeTransform` (+ (`KismetMathLibrary.MakeVector` -180.0 -510.0 50.0) (`self.PackSpawnLocation`)) (struct :`Yaw` -70.0)) "AdjustIfPossibleButAlwaysSpawn" "MultiplyWithRoot" null null))
    (:`then_3`
      (`|SpawnActorFromClass` "/Game/PAKK/Blueprints/Players/NPC/BP_NpcAI.BP_NpcAI_C" (`KismetMathLibrary.MakeTransform` (+ (`KismetMathLibrary.MakeVector` -740.0 -220.0 50.0) (`self.PackSpawnLocation`)) (struct :`Yaw` -190.0)) "AdjustIfPossibleButAlwaysSpawn" "MultiplyWithRoot" null null))))

(fn `UserConstructionScript`
  (`parent.UserConstructionScript`))